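; BP_WorldItem is a world pickup actor that gives an item to the interacting character's inventory.
; Its Interaction event calls AddItem on the character's BPInventory with the configured item class and either a fixed amount or a random one within a min/max range.
; The actor destroys itself on success and stays in the world on failure, printing a colored debug message either way.
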(event `/Game/Interface/BPI_interact.Interaction`
  (params (CharacterRef :type "/Game/ThirdPersonBP/Blueprints/ThirdPersonCharacter Object Reference"))
  (bind _addeditem_ (`/Game/Components/BP_Inventory_Component.AddItem` (`/Game/ThirdPersonBP/Blueprints/ThirdPersonCharacter.BP_Inventory` CharacterRef) (`self.ItemClass`) (select `bool` (`self.RandomAmount?`) :`false` (`self.AmountToAdd`) :`true` (`KismetMathLibrary.RandomIntegerInRange` (`self.MinRandomAmount`) (`self.MaxRandomAmount`)))))
  (if _addeditem_
    (`KismetSystemLibrary.PrintString` "AddedItem" true true (struct :`R` 0.29949 :`G` 1.0 :`A` 1.0))
    (`self.K2_DestroyActor`)
    (else
      (`KismetSystemLibrary.PrintString` "FailedToAdd" true true (struct :`R` 1.0 :`G` 0.001901 :`B` 0.30542 :`A` 1.0)))))

(fn `UserConstructionScript`)