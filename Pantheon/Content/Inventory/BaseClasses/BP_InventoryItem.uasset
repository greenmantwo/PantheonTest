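; Base inventory item class holding a row name and stack amount, with item data defined in DT_Items.
; Getters look up that row for item info, stackability, max stack size and remaining stack room, printing an error when the row is missing.
; OnUse and OnDrop are empty hooks, and SetAmount overwrites the amount despite its AmountToAdd parameter name.
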(fn `GetAmount`
  (returns (Amount :type Integer))
  (return (`self.Amount`)))

(fn `GetCanStack`
  (returns (`Can Stack?` :type Boolean))
  (bind _rowname (`self.RowName`))
  (bind _returnvalue (`|GetDataTableRow` "/Game/Structs/DataTables/DT_Items.DT_Items" _rowname)
    (:`then`
      (return (`.CanStack?_5_9833134F4EB883B7DF0467A56EBD4CC1` (break `/Game/Structs/FINventoryItem` _returnvalue))))
    (:`RowNotFound`
      (`KismetSystemLibrary.PrintString` null (`KismetStringLibrary.Concat_StrStr` "Row: " (`KismetStringLibrary.Conv_NameToString` _rowname) "not found"))
      (return false))))

(fn `GetInventoryItemInfo`
  (returns (InventoryItem :type "/Game/Structs/FINventoryItem Structure"))
  (bind _rowname (`self.RowName`))
  (bind _returnvalue (`|GetDataTableRow` "/Game/Structs/DataTables/DT_Items.DT_Items" _rowname)
    (:`then`
      (return _returnvalue))
    (:`RowNotFound`
      (`KismetSystemLibrary.PrintString` null (`KismetStringLibrary.Concat_StrStr` "Row: " (`KismetStringLibrary.Conv_NameToString` _rowname) "not found"))
      (return))))

(fn `GetItemInfo`
  (returns (`Item Info` :type "/Game/Structs/FItemInfo Structure"))
  (bind _rowname (`self.RowName`))
  (bind _returnvalue (`|GetDataTableRow` "/Game/Structs/DataTables/DT_Items.DT_Items" _rowname)
    (:`then`
      (return (break `/Game/Structs/FINventoryItem` _returnvalue)))
    (:`RowNotFound`
      (`KismetSystemLibrary.PrintString` null (`KismetStringLibrary.Concat_StrStr` "Row: " (`KismetStringLibrary.Conv_NameToString` _rowname) "not found"))
      (return))))

(fn `GetMaxStackAmount`
  (returns (`Out Row Max Stack Amount` :type Integer))
  (bind _rowname (`self.RowName`))
  (bind _returnvalue (`|GetDataTableRow` "/Game/Structs/DataTables/DT_Items.DT_Items" _rowname)
    (:`then`
      (return (`.MaxStackAmount_11_7A658DD54394CA67DBD955A926F70A32` (break `/Game/Structs/FINventoryItem` _returnvalue))))
    (:`RowNotFound`
      (`KismetSystemLibrary.PrintString` null (`KismetStringLibrary.Concat_StrStr` "Row: " (`KismetStringLibrary.Conv_NameToString` _rowname) "not found"))
      (return -1))))

(fn `GetRoomOnStack`
  (returns (ReturnValue :type Integer))
  (bind _rowname (`self.RowName`))
  (bind _returnvalue (`|GetDataTableRow` "/Game/Structs/DataTables/DT_Items.DT_Items" _rowname)
    (:`then`
      (return (- (`.MaxStackAmount_11_7A658DD54394CA67DBD955A926F70A32` (break `/Game/Structs/FINventoryItem` _returnvalue)) (`self.Amount`))))
    (:`RowNotFound`
      (`KismetSystemLibrary.PrintString` null (`KismetStringLibrary.Concat_StrStr` "Row: " (`KismetStringLibrary.Conv_NameToString` _rowname) "not found"))
      (return -1))))

(fn `OnDrop`)

(fn `OnUse`)

(fn `SetAmount`
  (params (`Amount ToAdd` :type Integer))
  (set `self.Amount` `Amount ToAdd`))