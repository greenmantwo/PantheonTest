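; Inventory component that holds a fixed number of item slots, each an item object, with empty slots filled by BP_InvItem_Empty placeholders created on BeginPlay.
; AddItem requires a free slot, tops up matching stackable items and puts overflow into a new object in the first empty slot.
; Slot getters and setters support SwapItems, which exchanges items within or between inventory components.
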(event `self.ReceiveBeginPlay`
  (`self.InitializeInventory`))

(fn `AddItem`
  (params (ItemToAdd :type "/Game/Inventory/BaseClasses/BP_InventoryItem Class Reference") (AmountToAdd :type Integer))
  (returns (`AddedItem?` :type Boolean))
  (locals (L_Class :type "/Game/Inventory/BaseClasses/BP_InventoryItem Class Reference") (L_Amount :type Integer) (L_OpenSpaces :type Integer :default 0) (L_Item :type "/Game/Inventory/BaseClasses/BP_InventoryItem Object Reference") (L_Index :type Integer))
  (bind (_hasspace_ _openspaces) (`self.HasSpaceInInventory`))
  (bind _l_item (`local.L_Item`))
  (bind _l_item_2 (`local.L_Item`))
  (bind _l_item_3 (`local.L_Item`))
  (set `local.L_Class` ItemToAdd)
  (set `local.L_Amount` AmountToAdd)
  (if _hasspace_
    (set `local.L_OpenSpaces` _openspaces)
    (for _array_element (`self.Inventory`)
      (if (== (`GameplayStatics.GetObjectClass` _array_element) (`local.L_Class`))
        (bind _output_get (set `local.L_Item` _array_element))
        (if (`/Game/Inventory/BaseClasses/BP_InventoryItem.GetCanStack` _output_get)
          (if (> (`/Game/Inventory/BaseClasses/BP_InventoryItem.GetRoomOnStack` (`local.L_Item`)) 0)
            (if (<= (+ (`/Game/Inventory/BaseClasses/BP_InventoryItem.GetAmount` _l_item_2) (`local.L_Amount`)) (`/Game/Inventory/BaseClasses/BP_InventoryItem.GetMaxStackAmount` _l_item_2))
              (`/Game/Inventory/BaseClasses/BP_InventoryItem.SetAmount` _l_item_3 (+ (`/Game/Inventory/BaseClasses/BP_InventoryItem.GetAmount` _l_item_3) (`local.L_Amount`)))
              (return true)
              (elif (> (`local.L_OpenSpaces`) 0)
                (set `local.L_Amount` (- (`local.L_Amount`) (`/Game/Inventory/BaseClasses/BP_InventoryItem.GetRoomOnStack` (`local.L_Item`))))
                (`/Game/Inventory/BaseClasses/BP_InventoryItem.SetAmount` _l_item (`/Game/Inventory/BaseClasses/BP_InventoryItem.GetMaxStackAmount` _l_item))
                (for (_array_element_2 _array_index) (`self.Inventory`) :!label _label
                  (if (== (`GameplayStatics.GetObjectClass` _array_element_2) "/Game/Inventory/Objects/BP_InvItem_Empty.BP_InvItem_Empty_C")
                    (set `local.L_Index` _array_index)
                    (break)
                    (else
                      (set `local.L_Index` -1))))
                (if (>= (`local.L_Index`) 0)
                  (bind _returnvalue (`|GenericCreateObject` (`local.L_Class`) self))
                  (`/Game/Inventory/BaseClasses/BP_InventoryItem.SetAmount` _returnvalue (`local.L_Amount`))
                  (`KismetArrayLibrary.Array_Set` (`self.Inventory`) (`local.L_Index`) _returnvalue)
                  (return true)
                  (else
                    (return false)))
                (else
                  (return false)))))
          (else
            (goto _label)))))
    (goto _label)
    (else
      (return false))))

(fn `GetInventory`
  (returns (Inventory :type "Array of /Game/Inventory/BaseClasses/BP_InventoryItem Object Reference"))
  (return (`self.Inventory`)))

(fn `GetItemInSlot`
  (params (Index :type Integer))
  (returns (Item :type "/Game/Inventory/BaseClasses/BP_InventoryItem Object Reference"))
  (bind _output (`|GetArrayItem` (`self.Inventory`) Index))
  (`/Engine/EditorBlueprintResources/StandardMacros.IsValid` _output
    (:`Is Valid`
      (return _output))
    (:`Is Not Valid`
      (return null))))

(fn `HasSpaceInInventory`
  (returns (`HasSpace?` :type Boolean) (OpenSpaces :type Integer))
  (locals (L_OpenSpaces :type Integer))
  (bind _l_openspaces (`local.L_OpenSpaces`))
  (for _array_element (`self.Inventory`)
    (if (== (`GameplayStatics.GetObjectClass` _array_element) "/Game/Inventory/Objects/BP_InvItem_Empty.BP_InvItem_Empty_C")
      (`/Engine/EditorBlueprintResources/StandardMacros.IncrementInt` (`local.L_OpenSpaces`))))
  (return (> _l_openspaces 0) _l_openspaces))

(fn `InitializeInventory`
  (`KismetArrayLibrary.Array_Clear` (`self.Inventory`))
  (for _ (range (`self.Slots`))
    (bind _returnvalue (`|GenericCreateObject` "/Game/Inventory/Objects/BP_InvItem_Empty.BP_InvItem_Empty_C" self))
    (`KismetArrayLibrary.Array_Add` (`self.Inventory`) _returnvalue)))

(fn `SetSlotInInventory`
  (params (Item :type "/Game/Inventory/BaseClasses/BP_InventoryItem Object Reference") (Index :type Integer))
  (returns (`Success?` :type Boolean))
  (if (<= Index (`KismetArrayLibrary.Array_LastIndex` (`self.Inventory`)))
    (`KismetArrayLibrary.Array_Set` (`self.Inventory`) Index Item)
    (return true)
    (else
      (return false))))

(fn `SwapItems`
  (params (FromInventory :type "/Game/Components/BP_Inventory_Component Object Reference") (FromIndex :type Integer) (ToInventory :type "/Game/Components/BP_Inventory_Component Object Reference") (ToIndex :type Integer))
  (locals (L_FromItem :type "/Game/Inventory/BaseClasses/BP_InventoryItem Object Reference") (L_ToItem :type "/Game/Inventory/BaseClasses/BP_InventoryItem Object Reference"))
  (set `local.L_FromItem` (`self.GetItemInSlot` FromInventory FromIndex))
  (set `local.L_ToItem` (`self.GetItemInSlot` ToInventory ToIndex))
  (`self.SetSlotInInventory` FromInventory (`local.L_ToItem`) FromIndex)
  (`self.SetSlotInInventory` ToInventory (`local.L_FromItem`) ToIndex))