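; Weather manager actor that runs the day/night clock, sun position and world temperature.
; Each tick it advances elapsed time from a start time, pitches the directional light by curve, updates the sky sphere and sends the time to the HUD.
; A looping timer derives temperature from a fluctuation curve around a base value.
; Night-based sun intensity fading exists but is never called.
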(event `self.ReceiveBeginPlay`
  (`|ExecutionSequence`
    (:`then_0`
      (`self.GetSunAndSky`))
    (:`then_1`
      (`self.SetSunIntensity`))
    (:`then_2`
      (`self.SetElapsedTimeBasedOnStartTime`))
    (:`then_3`
      (`KismetSystemLibrary.Delay` 0.0001)
      (`self.SetHudReference`))
    (:`then_4`
      (`self.StartUpdatingTemperature`))))

(event `self.ReceiveTick`
  (params (DeltaSeconds :type "Float (single-precision)"))
  (`|ExecutionSequence`
    (:`then_0`
      (`self.UpdateElapsedTime`))
    (:`then_1`
      (`self.UpdateSunPosition`))
    (:`then_2`
      (`self.UpdateCurrentTime`))))

(fn `DetermineCurrentTime`
  (returns (Time :type "/Game/Structs/FTime Structure"))
  (bind _returnvalue (`self.GetFractionOfDay`))
  (return (make `/Game/Structs/FTime` (`KismetMathLibrary.FTrunc` _returnvalue) (`KismetMathLibrary.FTrunc` (* (mod _returnvalue 1.0) 24.0)) (`KismetMathLibrary.FTrunc` (mod (* _returnvalue 1440.0) 60.0)))))

(fn `DetermineIfNight`
  (returns (ReturnValue :type Boolean))
  (bind (_days _hours) (break `/Game/Structs/FTime` (`self.CurrentTime`)))
  (return (or (< _hours (`self.SunUpTime`)) (>= _hours (`self.SunDownTime`)))))

(fn `FadeSun`
  (bind _lightcomponent (`Light.LightComponent` (`self.Sun`)))
  (`LightComponent.SetIntensity` _lightcomponent (`KismetMathLibrary.FClamp` (+ (`LightComponentBase.Intensity` _lightcomponent) (* (`GameplayStatics.GetWorldDeltaSeconds`) (/ 24.0 (`self.SecondsPerDay`)) (`self.SunIntensity`) (select `bool` (`self.DetermineIfNight`) :`false` 1.0 :`true` -1.0 :!type "Float (single-precision)"))) 0.0 (`self.SunIntensity`))))

(fn `GetFractionOfDay`
  (returns (ReturnValue :type "Float (double-precision)"))
  (return (/ (`self.ElapsedTime`) (`self.SecondsPerDay`))))

(fn `GetSunAndSky`
  (`/Engine/EditorBlueprintResources/StandardMacros.IsValid` (`self.Sun`)
    (:`Is Valid`
      _)
    (:`Is Not Valid`
      (bind _outactors (`GameplayStatics.GetAllActorsOfClass` "/Script/Engine.DirectionalLight"))
      (set `self.Sun` (`|GetArrayItem` _outactors))))
  (`/Engine/EditorBlueprintResources/StandardMacros.IsValid` (`self.Sky`)
    (:`Is Not Valid`
      (bind _outactors_2 (`GameplayStatics.GetAllActorsOfClass` "/Engine/EngineSky/BP_Sky_Sphere.BP_Sky_Sphere_C"))
      (set `self.Sky` (`|GetArrayItem` _outactors_2)))))

(fn `GetTimeAsSeconds`
  (params (Time :type "/Game/Structs/FTime Structure (by ref)"))
  (returns (ReturnValue :type Integer))
  (bind (_days _hours _minutes) (break `/Game/Structs/FTime` Time))
  (return (+ (* _days 86400) (* _hours 3600) (* _minutes 60))))

(fn `SetElapsedTimeBasedOnStartTime`
  (set `self.ElapsedTime` (* (`self.GetTimeAsSeconds` (`self.StartTime`)) (/ (`self.SecondsPerDay`) 86400.0))))

(fn `SetHudReference`
  (`/Engine/EditorBlueprintResources/StandardMacros.IsValid` (`self.HUDRef`)
    (:`Is Not Valid`
      (bind _asthird_person_character (cast `/Game/ThirdPersonBP/Blueprints/ThirdPersonCharacter` (`GameplayStatics.GetPlayerCharacter` 0)))
      (set `self.HUDRef` (`/Game/ThirdPersonBP/Blueprints/ThirdPersonCharacter.Game HUD Ref` _asthird_person_character)))))

(fn `SetSunIntensity`
  (set `self.SunIntensity` (`LightComponentBase.Intensity` (`Light.LightComponent` (`self.Sun`)))))

(fn `StartUpdatingTemperature`
  (`KismetSystemLibrary.K2_SetTimer` self "UpdateWorldTemperature" (/ 1.0 (`self.TemperatureUpdateRate`)) true))

(fn `UpdateCurrentTime`
  (bind _hudref (`self.HUDRef`))
  (bind _output_get (set `self.CurrentTime` (`self.DetermineCurrentTime`)))
  (`/Engine/EditorBlueprintResources/StandardMacros.IsValid` _hudref
    (:`Is Valid`
      (`/Game/UI/UI_GameHUD.SetTime` _hudref _output_get (`self.ClockType`)))))

(fn `UpdateElapsedTime`
  (set `self.ElapsedTime` (+ (`self.ElapsedTime`) (`GameplayStatics.GetWorldDeltaSeconds`))))

(fn `UpdateSunPosition`
  (`SceneComponent.K2_SetRelativeRotation` (`Light.LightComponent` (`self.Sun`)) (`KismetMathLibrary.MakeRotator` 0.0 (`CurveFloat.GetFloatValue` (`self.SunPitchCurve`) (* (`self.GetFractionOfDay`) 24.0)) 30.0) false false)
  (`/Engine/EngineSky/BP_Sky_Sphere.UpdateSunDirection` (`self.Sky`)))

(fn `UpdateWorldTemperature`
  (set `self.FinalWorldTemperature` (+ (* (`CurveFloat.GetFloatValue` (`self.TempFluctuationCurve`) (mod (`self.GetFractionOfDay`) 1.0)) (`self.WorldTemperatureVariation`)) (`self.BaseWorldTemperature`))))

(fn `UserConstructionScript`
  (set `self.SecondsPerDay` (* (`self.MinutesPerDay`) 60.0)))